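; Far wall for VR racquetball that reacts to ball hits by painting itself, rebounding the ball and awarding points.
; On BeginPlay it creates a render target for the wall material and a dynamic brush material.
; Each hit line-traces for the UV and draws the previous player's color into that target.
; It also sets a semi-random rebound velocity and scores for player two if that player is AI, otherwise player one.
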(event `self.ReceiveBeginPlay`
  (bind _asrbvrgame_state (cast `RBVRGameState` (`GameplayStatics.GetGameState`)))
  (set `self.GameMode` _asrbvrgame_state)
  (`self.PrepareWallMaterial`))

(event `self.WallMesh.OnComponentHit`
  (params (HitComponent :type "PrimitiveComponent Object Reference") (OtherActor :type "Actor Object Reference") (OtherComp :type "PrimitiveComponent Object Reference") (NormalImpulse :type "Vector Structure") (Hit :type "HitResult Structure (by ref)"))
  ;[1 1 1] On Collision With Wall
  (bind _asball (cast `Ball` OtherActor))
  (`self.HandleBallCollision` _asball Hit))

(fn `HandleBallCollision`
  (params (_Ball :type "Ball Object Reference") (_HitResult :type "HitResult Structure (by ref)"))
  (locals (Ball :type "Ball Object Reference") (HitResult :type "HitResult Structure"))
  (bind (_hitresult_bblockinghit _hitresult_binitialoverlap _hitresult_time _hitresult_distance _hitresult_location _hitresult_impactpoint) (`GameplayStatics.BreakHitResult` (`local.HitResult`)))
  (bind (_hitresult_bblockinghit_2 _hitresult_binitialoverlap_2 _hitresult_time_2 _hitresult_distance_2 _hitresult_location_2 _hitresult_impactpoint_2) (`GameplayStatics.BreakHitResult` (`local.HitResult`)))
  (bind (_maxvelocity_x _maxvelocity_y) (`KismetMathLibrary.BreakVector` (`self.MaxVelocity`)))
  (bind (_minvelocity_x _minvelocity_y) (`KismetMathLibrary.BreakVector` (`self.MinVelocity`)))
  (bind (_minvelocity_x_2 _minvelocity_y_2 _minvelocity_z) (`KismetMathLibrary.BreakVector` (`self.MinVelocity`)))
  (bind (_maxvelocity_x_2 _maxvelocity_y_2 _maxvelocity_z) (`KismetMathLibrary.BreakVector` (`self.MaxVelocity`)))
  (bind (_hitresult_bblockinghit_3 _hitresult_binitialoverlap_3 _hitresult_time_3 _hitresult_distance_3 _hitresult_location_3 _hitresult_impactpoint_3 _hitresult_normal _hitresult_impactnormal) (`GameplayStatics.BreakHitResult` (`local.HitResult`)))
  (bind _previousplayer (`Ball.PreviousPlayer` (`local.Ball`)))
  (bind _previousplayer_2 (`Ball.PreviousPlayer` (`local.Ball`)))
  (set `local.Ball` _Ball)
  (set `local.HitResult` _HitResult)
  (`|ExecutionSequence`
    (:`then_0`
      ;[1 1 1] Get Hit Position
      (bind (_hitlocation _hitnormal _bonename _outhit) (`PrimitiveComponent.K2_LineTraceComponent` (`self.WallMesh`) _hitresult_impactpoint_3 (* (- _hitresult_impactpoint_3 _hitresult_impactnormal) 10.0) true true))
      ;[1 1 1] Paint Wall the Color of the Previous Player who hit the wall.
      (`/Engine/EditorBlueprintResources/StandardMacros.IsValid` _previousplayer_2
        (:`Is Valid`
          (`self.PaintWall` (`GameplayStatics.FindCollisionUV` _outhit) 0.15 (`KismetMathLibrary.Conv_ColorToLinearColor` (`RBVRPlayer.PlayerColor` _previousplayer_2))))))
    (:`then_1`
      ;[1 1 1] Apply Semi-Random Rebound Velocity
      (bind _returnvalue (`Ball.GetBallVelocity` (`local.Ball`)))
      (`Ball.SetBallVelocity` (`local.Ball`) (`KismetMathLibrary.MakeVector` (`KismetMathLibrary.FClamp` (.x _returnvalue) _minvelocity_x_2 _maxvelocity_x_2) (`KismetMathLibrary.FClamp` (select `bool` (>= (`KismetMathLibrary.Abs` (.y _hitresult_impactpoint)) (`self.OuterEdgeThreshold`)) :`false` (* (.y _returnvalue) (`KismetMathLibrary.RandomFloatInRange` 1.0 2.0)) :`true` (* (`KismetMathLibrary.SignOfFloat` (- (.y _hitresult_impactpoint_2) (.y (`self.K2_GetActorLocation`)))) (`self.OuterEdgeReboundYValue`))) _minvelocity_y _maxvelocity_y) (`KismetMathLibrary.FClamp` (.z _returnvalue) _minvelocity_z _maxvelocity_z))))
    (:`then_2`
      ;[1 1 1] Apply points to player.
      (`/Engine/EditorBlueprintResources/StandardMacros.IsValid` _previousplayer ; Check if the ball had been hit by a player.
        (:`Is Valid`
          (if (`.bSuccess` (cast `AIPlayer` _previousplayer :!pure true))
            (`RBVRGameState.AddPlayerTwoScore` (`self.GameMode`) 1)
            (else
              (`RBVRGameState.AddPlayerOneScore` (`self.GameMode`) 1))))))))

(fn `PaintWall`
  (params (HitPosition :type "Vector2D Structure" :default (0.5 0.5)) (HitRadius :type "Float (double-precision)" :default 0.5) (HitColor :type "LinearColor Structure" :default (struct :`R` 1.0 :`A` 1.0)))
  (bind (_x _y) (`KismetMathLibrary.BreakVector2D` HitPosition))
  (`|ExecutionSequence`
    (:`then_0`
      (`MaterialInstanceDynamic.SetVectorParameterValue` (`self.BrushMaterial`) (`self.PARAMETER_NAME_HIT_POSITION`) (`KismetMathLibrary.MakeColor` _x _y)))
    (:`then_1`
      (`MaterialInstanceDynamic.SetScalarParameterValue` (`self.BrushMaterial`) (`self.PARAMETER_NAME_HIT_RADIUS`) HitRadius))
    (:`then_2`
      (`MaterialInstanceDynamic.SetVectorParameterValue` (`self.BrushMaterial`) (`self.PARAMETER_NAME_HIT_COLOR`) HitColor))
    (:`then_3`
      (`KismetRenderingLibrary.DrawMaterialToRenderTarget` (`self.RenderTarget`) (`self.BrushMaterial`)))))

(fn `PrepareWallMaterial`
  (bind _returnvalue (`KismetRenderingLibrary.CreateRenderTarget2D` 512 512))
  (set `self.RenderTarget` _returnvalue)
  (bind _returnvalue_2 (`KismetMaterialLibrary.CreateDynamicMaterialInstance` "/Game/RacquetBallVR/Materials/Mat_Painting.Mat_Painting"))
  (bind _output_get (set `self.WallMaterial` _returnvalue_2))
  (`MaterialInstanceDynamic.SetTextureParameterValue` _output_get (`self.PARAMETER_NAME_RENDER_TARGET`) (`self.RenderTarget`))
  (`PrimitiveComponent.SetMaterial` (`self.WallMesh`) 0 (`self.WallMaterial`))
  (bind _returnvalue_3 (`KismetMaterialLibrary.CreateDynamicMaterialInstance` "/Game/RacquetBallVR/Materials/Mat_Brush.Mat_Brush"))
  (set `self.BrushMaterial` _returnvalue_3))

(fn `UserConstructionScript`)