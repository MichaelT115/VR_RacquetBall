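; Racquetball VR ball that takes on the color of the player who hits it.
; The construction script puts a dynamic material instance on the mesh and starts the ball black.
; On BeginPlay it binds to the OnPlayerRegistered dispatcher, which passes the player's color to SetBallColor to update a material vector parameter, falling back to black for an invalid player.
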(event `self.ReceiveBeginPlay`
  ;[1 1 1] When the ball is hit by a player, it changes to match the player's color.
  (add `self.OnPlayerRegistered` (delegate `ChangeBallColor`)))

(event `ChangeBallColor` :!signature `self.OnPlayerRegistered`
  (params (Player :type "RBVRPlayer Object Reference"))
  ;[1 1 1] When the ball is hit by a player, it changes to match the player's color.
  (`/Engine/EditorBlueprintResources/StandardMacros.IsValid` Player
    (:`Is Valid`
      (`self.SetBallColor` (`KismetMathLibrary.Conv_ColorToLinearColor` (`RBVRPlayer.PlayerColor` Player))))
    (:`Is Not Valid`
      (`self.SetBallColor` (struct)))))

(fn `SetBallColor`
  (params (NewColor :type "LinearColor Structure"))
  (`MaterialInstanceDynamic.SetVectorParameterValue` (`self.SphereMaterial`) (`self.BALL_COLOR_PARAMETER`) NewColor))

(fn `UserConstructionScript`
  (bind _returnvalue (`KismetMaterialLibrary.CreateDynamicMaterialInstance` "/Game/RacquetBallVR/Materials/Mat_Ball.Mat_Ball"))
  (bind _output_get (set `self.SphereMaterial` _returnvalue))
  (`PrimitiveComponent.SetMaterial` (`self.Mesh`) 0 _output_get)
  (`self.SetBallColor` (struct)))