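; Racquetball ball actor that shows which player was last registered with it through its color.
; The construction script creates a dynamic material instance on the sphere and initializes its color to black.
; RegisterPlayer stores the given player as PreviousPlayer and passes that player's color to SetBallColor, which updates the material's color parameter.
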(fn `RegisterPlayer`
  (params (PreviousPlayer :type "/Game/RacquetBall/Blueprints/BP_PlayerPawn Object Reference"))
  (bind _output_get (set `self.PreviousPlayer` PreviousPlayer))
  (`self.SetBallColor` (`KismetMathLibrary.Conv_ColorToLinearColor` (`/Game/RacquetBall/Blueprints/BP_PlayerPawn.PlayerColor` _output_get))))

(fn `SetBallColor`
  (params (Color :type "LinearColor Structure"))
  (`MaterialInstanceDynamic.SetVectorParameterValue` (`self.SphereMaterial`) (`self.BALL_COLOR_PARAMETER`) Color))

(fn `UserConstructionScript`
  (bind _returnvalue (`KismetMaterialLibrary.CreateDynamicMaterialInstance` "/Game/RacquerBall2/Materials/Mat_Ball.Mat_Ball"))
  (bind _output_get (set `self.SphereMaterial` _returnvalue))
  (`PrimitiveComponent.SetMaterial` (`self.Sphere`) 0 _output_get)
  (`self.SetBallColor` (struct)))