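; BP_Wall is a racquetball wall that gets painted in the color of the ball's previous player on each hit.
; Construction creates a render target shown by the wall's dynamic material, plus a brush material instance.
; On a BP_Ball hit, a component trace yields the collision UV, where PaintWall draws the brush into the render target.
; It then clamps the rebound velocity, randomizing sideways speed or overriding it near the edges.
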(event `self.WallMesh.OnComponentHit`
  (params (HitComponent :type "PrimitiveComponent Object Reference") (OtherActor :type "Actor Object Reference") (OtherComp :type "PrimitiveComponent Object Reference") (NormalImpulse :type "Vector Structure") (Hit :type "HitResult Structure (by ref)"))
  (bind _y (.y (`.ImpactPoint` (`GameplayStatics.BreakHitResult` Hit))))
  (`|ExecutionSequence`
    (:`then_0`
      (bind _asbp_ball (cast `/Game/RacquetBall/Blueprints/BP_Ball` OtherActor))
      (bind _returnvalue (`self.K2_GetActorLocation` _asbp_ball))
      (bind (_hitlocation _hitnormal _bonename _outhit) (`PrimitiveComponent.K2_LineTraceComponent` (`self.WallMesh`) _returnvalue (- _returnvalue NormalImpulse) true true))
      (`self.PaintWall` (`GameplayStatics.FindCollisionUV` _outhit) 0.15 (`KismetMathLibrary.Conv_ColorToLinearColor` (`/Game/RacquetBall/Blueprints/BP_PlayerPawn.PlayerColor` (`/Game/RacquetBall/Blueprints/BP_Ball.PreviousPlayer` _asbp_ball)))))
    (:`then_1`
      (bind _sphere (`/Game/RacquetBall/Blueprints/BP_Ball.Sphere` _asbp_ball))
      (bind _returnvalue_2 (`PrimitiveComponent.GetPhysicsLinearVelocity` _sphere "None"))
      (`PrimitiveComponent.SetPhysicsLinearVelocity` _sphere (`KismetMathLibrary.MakeVector` (`KismetMathLibrary.FClamp` (.x _returnvalue_2) -750.0 -1500.0) (`KismetMathLibrary.FClamp` (select `bool` (>= (`KismetMathLibrary.Abs` _y) 180.0) :`false` (* (.y _returnvalue_2) (`KismetMathLibrary.RandomFloatInRange` 1.0 2.0)) :`true` (* (`KismetMathLibrary.SignOfFloat` _y) -200.0)) -200.0 200.0) (`KismetMathLibrary.FClamp` (.z _returnvalue_2) 500.0 750.0)) false "None"))))

(fn `PaintWall`
  (params (HitPosition :type "Vector2D Structure" :default (0.5 0.5)) (HitRadius :type "Float (double-precision)" :default 0.5) (HitColor :type "LinearColor Structure" :default (struct :`R` 1.0 :`A` 1.0)))
  (bind (_x _y) (`KismetMathLibrary.BreakVector2D` HitPosition))
  (`|ExecutionSequence`
    (:`then_0`
      (`MaterialInstanceDynamic.SetVectorParameterValue` (`self.BrushMaterial`) (`self.PARAMETER_NAME_HIT_POSITION`) (`KismetMathLibrary.MakeColor` _x _y)))
    (:`then_1`
      (`MaterialInstanceDynamic.SetScalarParameterValue` (`self.BrushMaterial`) (`self.PARAMETER_NAME_HIT_RADIUS`) HitRadius))
    (:`then_2`
      (`MaterialInstanceDynamic.SetVectorParameterValue` (`self.BrushMaterial`) (`self.PARAMETER_NAME_HIT_COLOR`) HitColor))
    (:`then_3`
      (`KismetRenderingLibrary.DrawMaterialToRenderTarget` (`self.RenderTarget`) (`self.BrushMaterial`)))))

(fn `UserConstructionScript`
  (bind _returnvalue (`KismetRenderingLibrary.CreateRenderTarget2D` 512 512))
  (set `self.RenderTarget` _returnvalue)
  (bind _returnvalue_2 (`KismetMaterialLibrary.CreateDynamicMaterialInstance` "/Game/RacquetBall/Materials/Mat_Painting.Mat_Painting"))
  (bind _output_get (set `self.WallMaterial` _returnvalue_2))
  (`MaterialInstanceDynamic.SetTextureParameterValue` _output_get (`self.PARAMETER_NAME_RENDER_TARGET`) (`self.RenderTarget`))
  (`PrimitiveComponent.SetMaterial` (`self.WallMesh`) 0 (`self.WallMaterial`))
  (bind _returnvalue_3 (`KismetMaterialLibrary.CreateDynamicMaterialInstance` "/Game/RacquetBall/Materials/Mat_Brush.Mat_Brush"))
  (set `self.BrushMaterial` _returnvalue_3))