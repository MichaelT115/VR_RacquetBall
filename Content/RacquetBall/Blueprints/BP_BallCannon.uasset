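; BP_BallCannon is a racquetball launcher that spawns and fires a single quarter-scale BP_Ball when play begins.
; FireBall teleports the ball to FirePosition and overrides the linear velocity of its physics sphere with FireVelocity.
; The construction script and Tick both move the Cannon component to FirePosition in world space, keeping it aligned with the launch point in editor and at runtime.
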(event `self.ReceiveBeginPlay`
  (bind _returnvalue (`|SpawnActorFromClass` "/Game/RacquetBall/Blueprints/BP_Ball.BP_Ball_C" (`KismetMathLibrary.MakeTransform` (0.0 0.0 0.0) (struct) (0.25 0.25 0.25)) "Undefined" "OverrideRootScale" null null))
  (`self.FireBall` _returnvalue))

(event `self.ReceiveTick`
  (params (DeltaSeconds :type "Float (single-precision)"))
  (`self.UpdateCannonPosition`))

(fn `FireBall`
  (params (Ball :type "/Game/RacquetBall/Blueprints/BP_Ball Object Reference"))
  (locals (SpawnedBall :type "/Game/RacquetBall/Blueprints/BP_Ball Object Reference"))
  (`self.K2_SetActorLocation` Ball (`self.FirePosition`) false true)
  (`PrimitiveComponent.SetPhysicsLinearVelocity` (`/Game/RacquetBall/Blueprints/BP_Ball.Sphere` Ball) (`self.FireVelocity`) false "None"))

(fn `UpdateCannonPosition`
  (`SceneComponent.K2_SetWorldLocation` (`self.Cannon`) (`self.FirePosition`) false false))

(fn `UserConstructionScript`
  (`self.UpdateCannonPosition`))