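; AI opponent pawn for racquetball that tracks the first BP_Ball in the level and registers itself as owner of its child-actor racquet.
; Each Tick it moves toward the current targets, then recomputes them from the ball's height and side.
; It holds a fixed X, stands offset from the ball within clamped Y bounds, and yaws toward that side.
; Movement is speed-capped without overshoot, while clamped paddle height and yaw are interpolated.
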(event `self.ReceiveBeginPlay`
  (`|ExecutionSequence`
    (:`then_0`
      (bind _outactors (`GameplayStatics.GetAllActorsOfClass` "/Game/RacquetBall/Blueprints/BP_Ball.BP_Ball_C"))
      (set `self.Ball` (`|GetArrayItem` _outactors)))
    (:`then_1`
      (bind _asbp_racquet (cast `/Game/RacquetBall/Blueprints/BP_Racquet` (`ChildActorComponent.ChildActor` (`self.Racquet`))))
      (set `/Game/RacquetBall/Blueprints/BP_Racquet.PlayerOwner` self _asbp_racquet))))

(event `self.ReceiveTick`
  (params (DeltaSeconds :type "Float (single-precision)"))
  (bind _left_right_front (`self.GetBallLeftRightFront`))
  (bind _returnvalue (`self.K2_GetActorLocation`))
  (bind _returnvalue_2 (`self.K2_GetActorRotation`))
  (bind _racquetholder (`self.RacquetHolder`))
  (bind _returnvalue_3 (- (`self.DesiredPosition`) _returnvalue))
  (bind _returnvalue_4 (`SceneComponent.K2_GetComponentLocation` _racquetholder))
  (bind (_returnvalue_x _returnvalue_y) (`KismetMathLibrary.BreakVector` (`self.K2_GetActorLocation` (`self.Ball`))))
  (bind (_returnvalue_x_2 _returnvalue_y_2 _returnvalue_z) (`KismetMathLibrary.BreakVector` (`self.K2_GetActorLocation` (`self.Ball`))))
  (`|ExecutionSequence`
    (:`then_0`
      (`self.K2_SetActorLocation` (+ _returnvalue (`KismetMathLibrary.ClampVectorSize` (* (`KismetMathLibrary.Normal` _returnvalue_3) (* DeltaSeconds (`self.Speed`))) 0.0 (`KismetMathLibrary.VSize` _returnvalue_3))) true))
    (:`then_1`
      (`SceneComponent.K2_SetWorldLocation` _racquetholder (`KismetMathLibrary.VInterpTo_Constant` _returnvalue_4 (`KismetMathLibrary.MakeVector` (.x _returnvalue_4) (.y _returnvalue_4) (`self.DesiredPaddleHeight`)) DeltaSeconds (`self.PaddleHeightInterpolant`)) true false))
    (:`then_2`
      (`self.K2_SetActorRotation` (`KismetMathLibrary.RInterpTo` _returnvalue_2 (`KismetMathLibrary.MakeRotator` (.roll _returnvalue_2) (.pitch _returnvalue_2) (`self.DesiredRotation`)) DeltaSeconds (`self.RotationSpeed`))))
    (:`then_3`
      (`|ExecutionSequence`
        (:`then_0`
          (`self.SetPaddleHeight` _returnvalue_z))
        (:`then_1`
          (set `self.DesiredRotation` (select `/Game/RacquetBall/ELeftRightFront` _left_right_front :`NewEnumerator0` 90.0 :`NewEnumerator2` -90.0 :!type "Float (single-precision)")))
        (:`then_2`
          (`self.SetDesiredPosition` (`KismetMathLibrary.MakeVector` (`self.xPos`) (+ _returnvalue_y (* (`self.DesiredDistanceFromBall`) (select `bool` (`|EnumEquality` _left_right_front "NewEnumerator0") :`false` 1.0 :`true` -1.0 :!type "Float (single-precision)"))))))))))

(fn `GetBallLeftRightFront`
  (returns (`Left Right Front` :type "/Game/RacquetBall/ELeftRightFront Enum"))
  (bind (_returnvalue_x _returnvalue_y) (`KismetMathLibrary.BreakVector` (`self.K2_GetActorLocation`)))
  (bind (_returnvalue_x_2 _returnvalue_y_2) (`KismetMathLibrary.BreakVector` (`self.K2_GetActorLocation` (`self.Ball`))))
  (bind _returnvalue (`KismetMathLibrary.SignOfFloat` (- _returnvalue_y _returnvalue_y_2)))
  (return (select `bool` (== _returnvalue 0.0) :`false` (select `bool` (< _returnvalue 0.0) :`false` "NewEnumerator2" :`true` "NewEnumerator0" :!type "/Game/RacquetBall/ELeftRightFront Enum") :`true` "NewEnumerator1")))

(fn `SetDesiredPosition`
  (params (DesiredPosition :type "Vector Structure"))
  (set `self.DesiredPosition` (`KismetMathLibrary.MakeVector` (.x DesiredPosition) (`KismetMathLibrary.FClamp` (.y DesiredPosition) -215.0 215.0) (.z DesiredPosition))))

(fn `SetDesiredSpeed`)

(fn `SetPaddleHeight`
  (params (_DesiredDesiredPaddleHeight :type "Float (double-precision)"))
  (set `self.DesiredPaddleHeight` (`KismetMathLibrary.FClamp` _DesiredDesiredPaddleHeight (`self.MinPaddleHeight`) (`self.MaxPaddleHeight`))))

(fn `UserConstructionScript`
  (`parent.UserConstructionScript`))