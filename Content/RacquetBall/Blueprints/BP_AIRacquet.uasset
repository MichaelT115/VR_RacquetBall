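; BP_AIRacquet is the AI opponent's racquet in the RacquetBall game, a child Blueprint that overrides how it returns the ball.
; On a ball collision it runs the parent handling, then replaces the ball sphere's physics velocity with a random vector, each axis drawn between the MinVelocity and MaxVelocity bounds.
; The file contains no movement or tracking logic, only this randomized return.
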(event `self.HandleBallCollision`
  (params (Ball :type "/Game/RacquetBall/Blueprints/BP_Ball Object Reference") (HitResult :type "HitResult Structure"))
  (bind (_maxvelocity_x _maxvelocity_y _maxvelocity_z) (`KismetMathLibrary.BreakVector` (`self.MaxVelocity`)))
  (bind (_minvelocity_x _minvelocity_y _minvelocity_z) (`KismetMathLibrary.BreakVector` (`self.MinVelocity`)))
  (`parent.HandleBallCollision` Ball (struct))
  (`PrimitiveComponent.SetPhysicsLinearVelocity` (`/Game/RacquetBall/Blueprints/BP_Ball.Sphere` Ball) (`KismetMathLibrary.MakeVector` (`KismetMathLibrary.RandomFloatInRange` _minvelocity_x _maxvelocity_x) (`KismetMathLibrary.RandomFloatInRange` _minvelocity_y _maxvelocity_y) (`KismetMathLibrary.RandomFloatInRange` _minvelocity_z _maxvelocity_z)) false "None"))

(fn `UserConstructionScript`
  (`parent.UserConstructionScript`))