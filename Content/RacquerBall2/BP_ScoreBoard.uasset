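; BP_ScoreBoard is the racquetball scoreboard, showing both players' scores and the game countdown time.
; On BeginPlay it casts the game state to RBVRGameState and binds to its score and time update events.
; Those events write the new values to the CountDown, PlayerOneScore and PlayerTwoScore texts, so display is event-driven without Tick.
; BeginPlay also adds one point to player one right after binding.
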(event `self.ReceiveBeginPlay`
  (bind _asrbvrgame_state (cast `RBVRGameState` (`GameplayStatics.GetGameState`)))
  (bind _output_get (set `self.RBVRGameState` _asrbvrgame_state))
  (add `RBVRGameState.OnScoreUpdate` _output_get (delegate `OnScoreUpdate`))
  (add `RBVRGameState.OnGameTimeUpdate` (`self.RBVRGameState`) (delegate `OnGameTimeUpdate`))
  (`RBVRGameState.AddPlayerOneScore` (`self.RBVRGameState`) 1))

(event `OnGameTimeUpdate`
  (params (GameCountDownTime :type "Float (double-precision)"))
  (`TextRenderComponent.K2_SetText` (`self.CountDown`) (`KismetTextLibrary.Conv_DoubleToText` GameCountDownTime "HalfToEven")))

(event `OnScoreUpdate`
  (params (PlayerOneScore :type Integer) (PlayerTwoScore :type Integer))
  (`|ExecutionSequence`
    (:`then_0`
      (`TextRenderComponent.K2_SetText` (`self.PlayerOneScore`) (`KismetTextLibrary.Conv_IntToText` PlayerOneScore)))
    (:`then_1`
      (`TextRenderComponent.K2_SetText` (`self.PlayerTwoScore`) (`KismetTextLibrary.Conv_IntToText` PlayerTwoScore)))))

(fn `UserConstructionScript`)